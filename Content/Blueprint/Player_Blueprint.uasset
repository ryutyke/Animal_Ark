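; Player character Blueprint for a 2D side-view game with movement, shooting, fishing, inventory, chests and recipe mixing.
; Input drives multi-jump, overlap-counted ladder climbing, ortho camera zoom, and missiles fired toward the mouse with a spawned track and reload delay.
; Tick keeps the held fishing actor beside the player and teleports falls back up, gating most actions via Moveable for three seconds.
; SetPlayerState picks idle, run or jump flipbooks, blocking ground states mid-jump.
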(event `self.ReceiveTick`
  (params (DeltaSeconds :type "Float (single-precision)"))
  (bind (_returnvalue_x _returnvalue_y _returnvalue_z) (`KismetMathLibrary.BreakVector` (`self.K2_GetActorLocation`)))
  (bind (_returnvalue_x_2 _returnvalue_y_2 _returnvalue_z_2) (`KismetMathLibrary.BreakVector` (`self.K2_GetActorLocation`)))
  (bind (_returnvalue_x_3 _returnvalue_y_3 _returnvalue_z_3) (`KismetMathLibrary.BreakVector` (`self.K2_GetActorLocation`)))
  (bind _fishing (`self.fishing`))
  (if (`self.moveable`)
    ;[1 1 1] 떨어지면 부활
    (if (<= _returnvalue_z_3 -500.0)
      (`self.K2_SetActorLocation` (-0.479828 0.0 1200.0))
      (set `self.moveable` false)
      (elif (`self.Isfishing`)
        (if (`self.direction`)
          (`self.K2_SetActorRotation` :`self` _fishing)
          (`self.K2_SetActorLocation` _fishing (`KismetMathLibrary.MakeVector` (+ _returnvalue_x 28.0) 1.0 (- _returnvalue_z 250.0)) false false)
          (else
            (`self.K2_SetActorRotation` _fishing (struct :`Yaw` 180.0) false)
            (`self.K2_SetActorLocation` _fishing (`KismetMathLibrary.MakeVector` (+ _returnvalue_x_2 -28.0) 1.0 (- _returnvalue_z_2 250.0)) false false)))))
    (else
      (`KismetSystemLibrary.Delay` 3.0)
      (set `self.moveable` true))))

(event `MakeRoute`
  ;[1 1 1] 돌덩이 구현관련
  (bind _returnvalue (`|SpawnActorFromClass` "/Game/Blueprint/Tower/Track_BluePrint.Track_BluePrint_C" (`self.GetTransform`) "Undefined" "OverrideRootScale" null null))
  (set `self.route` _returnvalue))

(event `InputAction|Shoot`
  (params (Key :type "Key Structure"))
  (bind _worldlocation (`PlayerController.DeprojectMousePositionToWorld` (`GameplayStatics.GetPlayerController` 0)))
  (:`Pressed`
    (if (`self.moveable`)
      ;[1 1 1] 돌덩이 구현관련
      (if (`self.isReload`)
        (`self.MakeRoute`)
        (`|SpawnActorFromClass` "/Game/Blueprint/Tower/NormalMissle_BluePrint.NormalMissle_BluePrint_C" (`self.GetTransform`) "Undefined" "OverrideRootScale" null (`self.route`) null (`KismetMathLibrary.MakeVector` (.x _worldlocation) 0.0 (.z _worldlocation)) null 0.0 null)
        (set `self.isReload` false)
        (`KismetSystemLibrary.Delay` (`self.fireRate`))
        (set `self.isReload` true)))))

(event `InputAction|Chest`
  (params (Key :type "Key Structure"))
  (:`Pressed`
    (bind _outactors (`GameplayStatics.GetAllActorsOfClass` "/Game/Blueprint/Structure/Chest_Blueprint.Chest_Blueprint_C"))
    (for _array_element _outactors
      (if (`self.IsOverlappingActor` _array_element self)
        (`/Game/InventorySystem/InventoryComponent.ToggleInventory` (`self.GetComponentByClass` _array_element "/Game/InventorySystem/InventoryComponent.InventoryComponent_C"))))))

(event `InputAction|fishing`
  (params (Key :type "Key Structure"))
  (:`Pressed`
    (if (`self.moveable`)
      (bind _returnvalue (`|SpawnActorFromClass` "/Game/Blueprint/fishing_Blueprint.fishing_Blueprint_C" (`KismetMathLibrary.MakeTransform` (0.0 0.0 0.0) (struct) (1.0 0.275 1.0)) "Undefined" "OverrideRootScale" null null))
      (set `self.fishing` _returnvalue)
      (set `self.IsFishing` true)))
  (:`Released`
    (if (`self.IsFishing`)
      (bind _outactors (`GameplayStatics.GetAllActorsOfClass` "/Game/Blueprint/fishing_Blueprint.fishing_Blueprint_C"))
      (for _array_element _outactors
        (`self.K2_DestroyActor` _array_element))
      (set `self.IsFishing` false))))

(event `InventoryFromUI`
  (`/Game/InventorySystem/InventoryComponent.ToggleInventory` (`self.InventoryComponent`) :!label _label))

(event `InputAction|Inventory`
  (params (Key :type "Key Structure"))
  (:`Pressed`
    (goto _label)))

(event `InputAxis|Mouse Wheel`
  (params (AxisValue :type "Float (single-precision)"))
  (`CameraComponent.SetOrthoWidth` (`self.Camera`) (`KismetMathLibrary.FClamp` (+ (* AxisValue -100.0) (`CameraComponent.OrthoWidth` (`self.Camera`))) 256.0 1024.0)))

(event `self.ReceiveActorBeginOverlap`
  (params (OtherActor :type "Actor Object Reference"))
  ;[1 1 1] 플레이어가 사다리 위에 있는지 확인하는 것(LadderOverlapCount가 0보다 크면 수직 이동 가능)
  (if (== (`GameplayStatics.GetObjectClass` OtherActor) "/Game/Blueprint/Structure/WoodLadder_Blueprint.WoodLadder_Blueprint_C")
    (set `self.LadderOverlapCount` (+ (`self.LadderOverlapCount`) 1))))

(event `self.ReceiveActorEndOverlap`
  (params (OtherActor :type "Actor Object Reference"))
  ;[1 1 1] 플레이어가 사다리 위에 있는지 확인하는 것(LadderOverlapCount가 0보다 크면 수직 이동 가능)
  (if (== (`GameplayStatics.GetObjectClass` OtherActor) "/Game/Blueprint/Structure/WoodLadder_Blueprint.WoodLadder_Blueprint_C")
    (set `self.LadderOverlapCount` (+ (`self.LadderOverlapCount`) -1))))

(event `InputAxis|Horizontal`
  (params (AxisValue :type "Float (single-precision)"))
  (if (`self.moveable`)
    (if (!= AxisValue 0.0)
      (if (> AxisValue 0.0)
        (set `self.direction` true)
        (`SceneComponent.K2_SetRelativeRotation` :`self` (`self.Sprite`))
        (else
          (set `self.direction` false)
          (`SceneComponent.K2_SetRelativeRotation` (`self.Sprite`) (struct :`Yaw` 180.0) false false)))
      (`self.AddMovementInput` (1.0 0.0 0.0) AxisValue)
      (`self.SetPlayerState` "NewEnumerator2")
      (else
        (`self.SetPlayerState` "NewEnumerator0")))))

(event `InputAxis|Vertical`
  (params (AxisValue :type "Float (single-precision)"))
  ;[1 1 1] 플레이어가 사다리 위에 있는지 확인하는 것(LadderOverlapCount가 0보다 크면 수직 이동 가능)
  (if (> AxisValue 0.0)
    (if (> (`self.LadderOverlapCount`) 0)
      (`self.LaunchCharacter` (0.0 0.0 100.0) false true))))

(event `InputAction|Jump`
  (params (Key :type "Key Structure"))
  (:`Pressed`
    (if (`self.moveable`)
      (if (>= (`self.MaxJumpCnt`) (`self.CurrentJumpCnt`))
        (set `self.CurrentJumpCnt` (+ (stale `self.OnLanded` _output_get) 1))
        (`self.LaunchCharacter` (0.0 0.0 400.0) false true)
        (`self.SetPlayerState` "NewEnumerator1")))))

(event `self.OnLanded`
  (params (Hit :type "HitResult Structure (by ref)"))
  (bind _output_get (set `self.CurrentJumpCnt` 0)))

(fn `Mix Item`
  (params (Recipe :type "Map of /Game/Blueprint/Resource_Enum Enum to Integer"))
  (returns (success :type Boolean))
  (bind _returnvalue (`self.GetComponentByClass` "/Game/InventorySystem/InventoryComponent.InventoryComponent_C"))
  (bind _mixable (`/Game/InventorySystem/InventoryComponent.IsMixable` _returnvalue Recipe))
  (if _mixable
    (`/Game/InventorySystem/InventoryComponent.Mix` _returnvalue Recipe))
  (return _mixable))

(fn `SetFlipbookByEnum`
  (`PaperFlipbookComponent.SetFlipbook` (`self.Sprite`) (select `/Game/Blueprint/HumanState_Enum` (`self.PlayerStateEnum`) :`NewEnumerator0` "/Game/Sprite/human/Player/player_idle.player_idle" :`NewEnumerator2` "/Game/Sprite/human/Player/player_run.player_run" :`NewEnumerator1` "/Game/Sprite/human/Player/player_jump.player_jump" :!type "PaperFlipbook Object Reference")))

(fn `SetPlayerState`
  (params (InputPlayerState :type "/Game/Blueprint/HumanState_Enum Enum" :default "NewEnumerator0") (Force :type Boolean))
  (locals (InputState :type "/Game/Blueprint/HumanState_Enum Enum"))
  (bind _returnvalue (== (`self.CurrentJumpCnt`) 0))
  (set `local.InputState` InputPlayerState)
  (if Force
    (set `self.PlayerStateEnum` (`local.InputState`))
    (else
      (switch `/Game/Blueprint/HumanState_Enum` (`local.InputState`)
        (:`NewEnumerator0`
          (if _returnvalue
            (set `self.PlayerStateEnum` (`local.InputState`) :!label _label)
            (`self.SetFlipbookByEnum`)))
        (:`NewEnumerator2`
          (if _returnvalue
            (goto _label)))
        (:`NewEnumerator1`
          (goto _label))))))

(fn `UserConstructionScript`)