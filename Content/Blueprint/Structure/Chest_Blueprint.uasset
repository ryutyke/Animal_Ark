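; Chest actor that holds a preset set of items in an inventory component.
; On BeginPlay it copies its Items array slot by slot into the component's Inventory.
; While the inventory is open, Tick looks up the Player_Blueprint actor and toggles the inventory closed once that player no longer overlaps the chest.
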(event `self.ReceiveBeginPlay`
  (`parent.ReceiveBeginPlay`)
  (for (_array_element _array_index) (`self.Items`)
    (`KismetArrayLibrary.Array_Set` (`/Game/InventorySystem/InventoryComponent.Inventory` (`self.InventoryComponent`)) _array_index _array_element)))

(event `self.ReceiveTick`
  (params (DeltaSeconds :type "Float (single-precision)"))
  (bind _inventorycomponent (`self.InventoryComponent`))
  (`parent.ReceiveTick` DeltaSeconds)
  (if (`/Game/InventorySystem/InventoryComponent.IsOpened` _inventorycomponent)
    (bind _returnvalue (`GameplayStatics.GetActorOfClass` "/Game/Blueprint/Player_Blueprint.Player_Blueprint_C"))
    (if (not (`self.IsOverlappingActor` _returnvalue))
      (`/Game/InventorySystem/InventoryComponent.ToggleInventory` _inventorycomponent))))

(fn `UserConstructionScript`
  (`parent.UserConstructionScript`))