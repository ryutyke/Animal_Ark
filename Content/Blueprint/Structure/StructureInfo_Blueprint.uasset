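; StructureInfo is a lookup Blueprint holding the build cost and durability of each placeable structure, such as blocks, ladders, chests, towers, fences and cranes.
; GetStructureCost uses a Select on the structure enum to return a map of resource types to required amounts.
; GetStructureMaxHP uses the same Select pattern to return each structure's maximum health.
; The event graph and construction script are empty, so all data is hardcoded in these two functions.
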(fn `GetStructureCost`
  (params (Structure :type "/Game/Blueprint/Structure/Structure_Enum Enum" :default "NewEnumerator0"))
  (returns (Cost :type "Map of /Game/Blueprint/Resource_Enum Enum to Integer"))
  (return (select `/Game/Blueprint/Structure/Structure_Enum` Structure :`NewEnumerator0` (`|MakeMap` "NewEnumerator0" 2 :!type "/Game/Blueprint/Resource_Enum Enum") :`NewEnumerator2` (`|MakeMap` "NewEnumerator0" 5 :!type "/Game/Blueprint/Resource_Enum Enum") :`NewEnumerator3` (`|MakeMap` "NewEnumerator0" 10 "NewEnumerator3" 3 :!type "/Game/Blueprint/Resource_Enum Enum") :`NewEnumerator1` (`|MakeMap` "NewEnumerator0" 12 "NewEnumerator1" 5 :!type "/Game/Blueprint/Resource_Enum Enum") :`NewEnumerator9` (`|MakeMap` "NewEnumerator3" 20 "NewEnumerator5" 3 :!type "/Game/Blueprint/Resource_Enum Enum") :`NewEnumerator4` (`|MakeMap` "NewEnumerator1" 2 :!type "/Game/Blueprint/Resource_Enum Enum") :`NewEnumerator5` (`|MakeMap` "NewEnumerator3" 2 :!type "/Game/Blueprint/Resource_Enum Enum") :`NewEnumerator6` (`|MakeMap` "NewEnumerator4" 2 :!type "/Game/Blueprint/Resource_Enum Enum") :`NewEnumerator7` (`|MakeMap` "NewEnumerator5" 2 :!type "/Game/Blueprint/Resource_Enum Enum") :`NewEnumerator8` (`|MakeMap` "NewEnumerator0" 10 "NewEnumerator3" 5 :!type "/Game/Blueprint/Resource_Enum Enum") :`NewEnumerator10` (`|MakeMap` "NewEnumerator1" 12 "NewEnumerator4" 8 :!type "/Game/Blueprint/Resource_Enum Enum"))))

(fn `GetStructureMaxHP`
  (params (Structure :type "/Game/Blueprint/Structure/Structure_Enum Enum" :default "NewEnumerator0"))
  (returns (MaxHP :type "Float (double-precision)"))
  (return (select `/Game/Blueprint/Structure/Structure_Enum` Structure :`NewEnumerator0` 100.0 :`NewEnumerator2` 40.0 :`NewEnumerator3` 60.0 :`NewEnumerator1` 80.0 :`NewEnumerator9` 180.0 :`NewEnumerator4` 160.0 :`NewEnumerator5` 180.0 :`NewEnumerator6` 200.0 :`NewEnumerator7` 260.0 :`NewEnumerator8` 120.0 :`NewEnumerator10` 200.0 :!type "Float (single-precision)")))

(fn `UserConstructionScript`)