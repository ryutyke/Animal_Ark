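; Crane actor that repeatedly spawns a Craning_Blueprint load and carries it hanging below itself.
; While IsCraning is set, Tick pins the current load at a fixed offset under the crane.
; When IsCraning is false and no cooldown is running, it spawns a new half-height load with itself as OwnerCrane.
; A three-second cooldown starts at each spawn; nothing here clears IsCraning.
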(event `self.ReceiveActorBeginOverlap`
  (params (OtherActor :type "Actor Object Reference"))
  (`parent.ReceiveActorBeginOverlap` OtherActor))

(event `self.ReceiveTick`
  (params (DeltaSeconds :type "Float (single-precision)"))
  (bind (_returnvalue_x _returnvalue_y _returnvalue_z) (`KismetMathLibrary.BreakVector` (`self.K2_GetActorLocation`)))
  (bind (_returnvalue_x_2 _returnvalue_y_2 _returnvalue_z_2) (`KismetMathLibrary.BreakVector` (`self.K2_GetActorLocation`)))
  (`parent.ReceiveTick` DeltaSeconds)
  (if (`self.IsCraning`)
    (`self.K2_SetActorLocation` (`self.CraningActor`) (`KismetMathLibrary.MakeVector` _returnvalue_x _returnvalue_y (- _returnvalue_z 220.0)) false false)
    (elif (not (`self.IsCooltime`))
      (set `self.IsCraning` true)
      (bind _returnvalue (`|SpawnActorFromClass` "/Game/Blueprint/craning_Blueprint.craning_Blueprint_C" (`KismetMathLibrary.MakeTransform` (`KismetMathLibrary.MakeVector` _returnvalue_x_2 _returnvalue_y_2 (- _returnvalue_z_2 220.0)) (struct) (1.0 1.0 0.5)) "Undefined" "OverrideRootScale" null self null))
      (set `self.CraningActor` _returnvalue)
      (set `self.IsCooltime` true)
      (`KismetSystemLibrary.Delay` 3.0)
      (set `self.IsCooltime` false))))

(fn `UserConstructionScript`
  (`parent.UserConstructionScript`))