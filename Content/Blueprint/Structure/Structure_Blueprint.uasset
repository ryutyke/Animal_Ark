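; Destructible sprite structure block that tracks its own HP and sits on a grid position under a parent Arc_Blueprint.
; Damaged subtracts HP and plays a collision sound; at zero it reports its GridPos to the attached parent, plays a crush sound and destroys itself.
; Below half HP, Tick repeatedly fades the sprite's alpha out and wraps it back, producing a blinking warning.
; An HP-based red tint is left unconnected.
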(event `self.ReceiveBeginPlay`
  (set `self.HP` (`self.MaxHP`)))

(event `SetMaxHP`
  (params (Value :type "Float (double-precision)"))
  (bind _output_get (set `self.MaxHP` Value))
  (set `self.HP` _output_get))

(event `self.ReceiveTick`
  (params (DeltaSeconds :type "Float (single-precision)"))
  (bind _papersprite (`self.PaperSprite`))
  (bind (_spritecolor_r _spritecolor_g _spritecolor_b _spritecolor_a) (break `LinearColor` (`PaperSpriteComponent.SpriteColor` (`self.PaperSprite`))))
  (bind _returnvalue (- _spritecolor_a (* (`GameplayStatics.GetWorldDeltaSeconds`) 1.0)))
  (if (< (/ (`self.HP`) (`self.MaxHP`)) 0.5)
    (if (> _returnvalue 0.0)
      (`PaperSpriteComponent.SetSpriteColor` _papersprite (make `LinearColor` 1.0 1.0 1.0 _returnvalue))
      (else
        (`PaperSpriteComponent.SetSpriteColor` _papersprite (make `LinearColor` 1.0 1.0 1.0 (+ _returnvalue 1.0)))))))

(event `Damaged`
  (params (Damage :type "Float (double-precision)"))
  (bind _output_get (set `self.HP` (- (`self.HP`) Damage)))
  (if (<= _output_get 0.0)
    (bind _asarc_blueprint (cast `/Game/Blueprint/Arc_Blueprint` (`self.GetAttachParentActor`)))
    (`/Game/Blueprint/Arc_Blueprint.StructureDestroyed` _asarc_blueprint (`self.GridPos`))
    (`GameplayStatics.PlaySound2D` "/Game/Sound/block_crush.block_crush" 1.0 1.0 0.0 null null)
    (`self.K2_DestroyActor`)
    (else
      (`GameplayStatics.PlaySound2D` "/Game/Sound/block_collision.block_collision" 1.0 1.0 0.0 null null))))

(fn `UserConstructionScript`)