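; ItemSpawner is an actor that continuously spawns resource items and, occasionally, animals at a fixed X/Y position with a random height.
; Tick rolls between the two groups, picking resources by rarity weight from Gold to Wood, or one of five animals with equal odds.
; A Spawn flag gates Tick through a random Delay after each spawn, and resource picks also record their name in ItemToRespawn.
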(event `self.ReceiveTick`
  (params (DeltaSeconds :type "Float (single-precision)"))
  (bind _itemspawnpos (`self.ItemSpawnPos`))
  (bind _itemspawnpos_2 (`self.ItemSpawnPos`))
  (if (`self.Spawn`)
    (set `self.SpawnDelay` (`KismetMathLibrary.RandomFloatInRange` 0.5 2.0))
    (bind _output_get (set `self.ItemOrAnimal` (`KismetMathLibrary.RandomFloat`)))
    (set `self.ItemSpawnPos` (`KismetMathLibrary.MakeVector` -1123.997681 0.000366 (`KismetMathLibrary.Conv_IntToDouble` (`KismetMathLibrary.RandomIntegerInRange` -250 -150))))
    (if (< _output_get 0.9)
      (bind _output_get_2 (set `self.ItemType` (`KismetMathLibrary.RandomFloat`)))
      (if (< _output_get_2 0.05)
        ;[1 1 1] 없어도됨
        (set `self.ItemToRespawn` "Gold")
        (`|SpawnActorFromClass` "/Game/Blueprint/ItemBP/Gold.Gold_C" (`KismetMathLibrary.Conv_VectorToTransform` _itemspawnpos_2) "Undefined" "OverrideRootScale" null null)
        (elif (< _output_get_2 0.15)
          (set `self.ItemToRespawn` "Silver")
          (`|SpawnActorFromClass` "/Game/Blueprint/ItemBP/Silver.Silver_C" (`KismetMathLibrary.Conv_VectorToTransform` _itemspawnpos_2) "Undefined" "OverrideRootScale" null null)
          (elif (< _output_get_2 0.35)
            (set `self.ItemToRespawn` "Cooper")
            (`|SpawnActorFromClass` "/Game/Blueprint/ItemBP/Copper.Copper_C" (`KismetMathLibrary.Conv_VectorToTransform` _itemspawnpos_2) "Undefined" "OverrideRootScale" null null)
            (elif (< _output_get_2 0.65)
              (set `self.ItemToRespawn` "Stone")
              (`|SpawnActorFromClass` "/Game/Blueprint/ItemBP/Stone.Stone_C" (`KismetMathLibrary.Conv_VectorToTransform` _itemspawnpos_2) "Undefined" "OverrideRootScale" null null)
              (else
                (set `self.ItemToRespawn` "Wood")
                (`|SpawnActorFromClass` "/Game/Blueprint/ItemBP/Wood.Wood_C" (`KismetMathLibrary.Conv_VectorToTransform` _itemspawnpos_2) "Undefined" "OverrideRootScale" null null))))))
      (set `self.Spawn` false)
      (`KismetSystemLibrary.Delay` (`self.SpawnDelay`))
      (set `self.Spawn` true)
      (else
        (bind _output_get_3 (set `self.AnimalType` (`KismetMathLibrary.RandomFloat`)))
        (if (< _output_get_3 0.2)
          (`|SpawnActorFromClass` "/Game/Blueprint/Animal/Dog.Dog_C" (`KismetMathLibrary.Conv_VectorToTransform` _itemspawnpos) "Undefined" "OverrideRootScale" null null)
          (elif (< _output_get_3 0.4)
            (`|SpawnActorFromClass` "/Game/Blueprint/Animal/Cat.Cat_C" (`KismetMathLibrary.Conv_VectorToTransform` _itemspawnpos) "Undefined" "OverrideRootScale" null null)
            (elif (< _output_get_3 0.6)
              (`|SpawnActorFromClass` "/Game/Blueprint/Animal/Elephant.Elephant_C" (`KismetMathLibrary.Conv_VectorToTransform` _itemspawnpos) "Undefined" "OverrideRootScale" null null)
              (elif (< _output_get_3 0.8)
                (`|SpawnActorFromClass` "/Game/Blueprint/Animal/Giraffe.Giraffe_C" (`KismetMathLibrary.Conv_VectorToTransform` _itemspawnpos) "Undefined" "OverrideRootScale" null null)
                (else
                  (`|SpawnActorFromClass` "/Game/Blueprint/Animal/Lion.Lion_C" (`KismetMathLibrary.Conv_VectorToTransform` _itemspawnpos) "Undefined" "OverrideRootScale" null null))))))
        (set `self.Spawn` false)
        (`KismetSystemLibrary.Delay` (`self.SpawnDelay`))
        (set `self.Spawn` true)))))

(event `self.ReceiveDestroyed`
  (set `self.Spawn` false))

(fn `UserConstructionScript`)