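; Item actor Blueprint that can be picked up into an interacting actor's inventory.
; Interact adds one unit of its ItemStructure through the interacter's InventoryComponent and destroys the actor only if that succeeds.
; Each Tick it drifts along world X by a random Speed chosen at BeginPlay, unscaled by delta time.
; UseItem is a stub that always returns true.
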(event `self.ReceiveBeginPlay`
  (set `self.speed` (`KismetMathLibrary.RandomFloat`)))

(event `self.ReceiveTick`
  (params (DeltaSeconds :type "Float (single-precision)"))
  (`self.K2_SetActorLocation` (+ (`self.K2_GetActorLocation`) (`KismetMathLibrary.MakeVector` (`self.speed`)))))

(event `/Game/InventorySystem/Interact_Interface.Interact`
  (params (Interacter :type "Actor Object Reference"))
  (bind _success (`/Game/InventorySystem/InventoryComponent.AddToInventory` (`self.GetComponentByClass` Interacter "/Game/InventorySystem/InventoryComponent.InventoryComponent_C") (make `/Game/InventorySystem/SlotStructure` (`self.ItemStructure`) 1)))
  (if _success
    (`self.K2_DestroyActor`)))

(fn `UseItem`
  (returns (Success :type Boolean))
  (return true))

(fn `UserConstructionScript`)