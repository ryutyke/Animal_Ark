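; Normal missile tower Blueprint for a tower defense game that fires at enemies once a target location has been set.
; Clicking it tints the sprite and opens a missile-setup widget, from which Tick copies the selected location.
; When reloaded, Tick acquires a target or spawns a track actor as the route and a projectile carrying route, target, location and range.
; A FireRate delay gates each shot.
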(event `self.ReceiveBeginPlay`
  (set `self.HP` 80.0))

(event `MakeRoute`
  (bind _returnvalue (`|SpawnActorFromClass` "/Game/Blueprint/Tower/Track_BluePrint.Track_BluePrint_C" (`self.GetTransform`) "Undefined" "OverrideRootScale" null null))
  (set `self.route` _returnvalue))

(event `Shoot`
  (`|SpawnActorFromClass` "/Game/Blueprint/Tower/NormalMissle_BluePrint.NormalMissle_BluePrint_C" (`self.GetTransform`) "Undefined" "OverrideRootScale" null (`self.route`) self (`self.selectLoc`) (`self.Target`) (`SphereComponent.SphereRadius` (`self.attackRange`)) null)
  (set `self.isReload` false)
  (`KismetSystemLibrary.Delay` (`self.fireRate`))
  (set `self.isReload` true))

(event `self.ReceiveTick`
  (params (DeltaSeconds :type "Float (single-precision)"))
  (bind _mywidget (`self.mywidget`))
  (if (and (`self.isReload`) (`KismetMathLibrary.NotEqualExactly_VectorVector` (`self.selectLoc`)) (`KismetSystemLibrary.IsValid` (`self.mywidget`)))
    (if (`KismetSystemLibrary.IsValid` (`self.Target`))
      (`self.MakeRoute`)
      (`self.Shoot`)
      (elif (not (`self.checkTarget`))
        (`self.TargetNewEnemy`)))
    (elif (`KismetSystemLibrary.IsValid` _mywidget)
      (set `self.selectLoc` (`/Game/Blueprint/Tower/SetNormalMissleWidget_BluePrint.selectLoc` _mywidget)))))

(event `self.ReceiveActorOnClicked`
  (params (ButtonPressed :type "Key Structure"))
  (`PaperSpriteComponent.SetSpriteColor` (`self.RenderComponent`) (struct :`R` 0.335 :`G` 0.382 :`B` 0.451 :`A` 1.0))
  (bind _returnvalue (`|CreateWidget` "/Game/Blueprint/Tower/SetNormalMissleWidget_BluePrint.SetNormalMissleWidget_BluePrint_C" null (`self.K2_GetActorLocation`) (`SphereComponent.SphereRadius` (`self.attackRange`)) self))
  (bind _output_get (set `self.mywidget` _returnvalue))
  (`UserWidget.AddToViewport` _output_get 0))

(fn `UserConstructionScript`
  (`parent.UserConstructionScript`))