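; Tower Blueprint that tracks an enemy target within its AttackRange sphere and takes damage when enemies hit it.
; AttackRange overlaps set Target when none is valid and clear it when that actor leaves.
; TargetNewEnemy sphere-traces that radius and uses FindNewEnemy to pick the closest enemy, holding CheckTarget true for a short delay.
; Enemies touching Collision receive damage, pass their Damage value to the tower's Damaged call, then are destroyed.
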(event `TargetNewEnemy`
  (bind _returnvalue (`self.K2_GetActorLocation`))
  (set `self.checkTarget` true)
  (bind (_outhits _returnvalue_2) (`KismetSystemLibrary.SphereTraceMultiForObjects` _returnvalue (- _returnvalue (0.0 0.0 1.0)) (`SphereComponent.SphereRadius` (`self.attackRange`)) (`|MakeArray` "ObjectTypeQuery10" :!type "EObjectTypeQuery Enum")))
  (if _returnvalue_2
    (bind _newenemy (`self.FindNewEnemy` _outhits))
    (`/Engine/EditorBlueprintResources/StandardMacros.IsValid` _newenemy
      (:`Is Valid`
        (set `self.Target` _newenemy))
      (:`Is Not Valid`
        _)))
  (`KismetSystemLibrary.Delay` 0.25)
  (set `self.checkTarget` false))

(event `self.attackRange.OnComponentBeginOverlap`
  (params (OverlappedComponent :type "PrimitiveComponent Object Reference") (OtherActor :type "Actor Object Reference") (OtherComp :type "PrimitiveComponent Object Reference") (OtherBodyIndex :type Integer) (bFromSweep :type Boolean) (SweepResult :type "HitResult Structure (by ref)"))
  (`/Engine/EditorBlueprintResources/StandardMacros.IsValid` (`self.Target`)
    (:`Is Not Valid`
      (bind _asenemy_blue_print (cast `/Game/Blueprint/Enemy/Enemy_BluePrint` OtherActor))
      (set `self.Target` _asenemy_blue_print))))

(event `self.attackRange.OnComponentEndOverlap`
  (params (OverlappedComponent :type "PrimitiveComponent Object Reference") (OtherActor :type "Actor Object Reference") (OtherComp :type "PrimitiveComponent Object Reference") (OtherBodyIndex :type Integer))
  (if (== OtherActor (`self.Target`))
    (set `self.Target` null)))

(event `self.collision.OnComponentBeginOverlap`
  (params (OverlappedComponent :type "PrimitiveComponent Object Reference") (OtherActor :type "Actor Object Reference") (OtherComp :type "PrimitiveComponent Object Reference") (OtherBodyIndex :type Integer) (bFromSweep :type Boolean) (SweepResult :type "HitResult Structure (by ref)"))
  (bind _overlapenemy (`self.overlapEnemy`))
  (bind _asenemy_blue_print (cast `/Game/Blueprint/Enemy/Enemy_BluePrint` OtherActor))
  (bind _output_get (set `self.overlapEnemy` _asenemy_blue_print))
  (`GameplayStatics.ApplyDamage` _output_get 10.0)
  (`/Engine/EditorBlueprintResources/StandardMacros.IsValid` _overlapenemy
    (:`Is Valid`
      (`self.Damaged` (`/Game/Blueprint/Enemy/Enemy_BluePrint.damage` _overlapenemy))
      (`self.K2_DestroyActor` _overlapenemy))))

(fn `FindNewEnemy`
  (params (Hits :type "Array of HitResult Structure"))
  (returns (NewEnemy :type "/Game/Blueprint/Enemy/Enemy_BluePrint Object Reference"))
  (locals (enemy :type "/Game/Blueprint/Enemy/Enemy_BluePrint Object Reference") (distance :type "Float (double-precision)"))
  (for _array_element Hits
    (bind (_bblockinghit _binitialoverlap _time _distance _location _impactpoint _normal _impactnormal _physmat _hitactor) (`GameplayStatics.BreakHitResult` _array_element))
    (bind _asenemy_blue_print (cast `/Game/Blueprint/Enemy/Enemy_BluePrint` _hitactor))
    (`/Engine/EditorBlueprintResources/StandardMacros.IsValid` (`local.enemy`)
      (:`Is Valid`
        (bind _returnvalue (`KismetMathLibrary.VSize` (- (`self.K2_GetActorLocation`) (`self.K2_GetActorLocation` _hitactor))))
        (if (< _returnvalue (`local.distance`))
          (set `local.enemy` _asenemy_blue_print)
          (set `local.distance` _returnvalue)))
      (:`Is Not Valid`
        (set `local.enemy` _asenemy_blue_print)
        (set `local.distance` _returnvalue))))
  (return (`local.enemy`)))

(fn `UserConstructionScript`)