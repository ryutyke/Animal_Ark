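; Homing missile projectile, apparently fired by a guided tower, that chases a target enemy and deals damage on overlap.
; Each Tick it moves at constant speed toward the target, or toward its last known location if the target is invalid, self-destructing on arrival there.
; Overlap damages and destroys it on the target enemy or another guided tower, ignoring its own tower.
; Other structures take damage without stopping the missile.
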(event `self.ReceiveBeginPlay`
  (set `self.damage` 10.0))

(event `self.ReceiveTick`
  (params (DeltaSeconds :type "Float (single-precision)"))
  (bind _targetenemy (`self.TargetEnemy`))
  (bind _returnvalue (`self.K2_GetActorLocation` _targetenemy))
  (`/Engine/EditorBlueprintResources/StandardMacros.IsValid` _targetenemy
    (:`Is Valid`
      (set `self.lastKnownLoc` _returnvalue)
      (`self.K2_SetActorLocation` (`KismetMathLibrary.VInterpTo_Constant` (`self.K2_GetActorLocation`) _returnvalue DeltaSeconds (`self.speed`))))
    (:`Is Not Valid`
      (if (< (`KismetMathLibrary.VSize` (- (`self.K2_GetActorLocation`) (`self.lastKnownLoc`))) 20.0)
        (`self.K2_DestroyActor`)
        (else
          (`self.K2_SetActorLocation` (`KismetMathLibrary.VInterpTo_Constant` (`self.K2_GetActorLocation`) (`self.lastKnownLoc`) DeltaSeconds (`self.speed`))))))))

(event `self.Collision.OnComponentBeginOverlap`
  (params (OverlappedComponent :type "PrimitiveComponent Object Reference") (OtherActor :type "Actor Object Reference") (OtherComp :type "PrimitiveComponent Object Reference") (OtherBodyIndex :type Integer) (bFromSweep :type Boolean) (SweepResult :type "HitResult Structure (by ref)"))
  (bind _targetenemy (`self.TargetEnemy`))
  (bind _asstructure_blueprint (cast `/Game/Blueprint/Structure/Structure_Blueprint` OtherActor)
    (:`then`
      (bind _asguided_tower_blue_print (cast `/Game/Blueprint/Tower/GuidedTower_BluePRint` _asstructure_blueprint)
        (:`then`
          (if (!= (`self.selfTower`) _asguided_tower_blue_print)
            (`/Game/Blueprint/Structure/Structure_Blueprint.Damaged` _asguided_tower_blue_print (`self.damage`))
            (`self.K2_DestroyActor`)))
        (:`CastFailed`
          (`/Game/Blueprint/Structure/Structure_Blueprint.Damaged` _asstructure_blueprint (`self.damage`)))))
    (:`CastFailed`
      (bind _asenemy_blue_print (cast `/Game/Blueprint/Enemy/Enemy_BluePrint` OtherActor))
      (if (== _asenemy_blue_print _targetenemy)
        (`GameplayStatics.ApplyDamage` _targetenemy (`self.damage`))
        (set `self.isCollide` true)
        (`self.K2_DestroyActor`)))))

(fn `UserConstructionScript`
  (`parent.UserConstructionScript`))