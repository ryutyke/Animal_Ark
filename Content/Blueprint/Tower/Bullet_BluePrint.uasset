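; Tower bullet actor that flies along an arched spline toward a point derived from the mouse cursor, then destroys itself.
; On BeginPlay it sets Damage and computes the end point from the deprojected cursor position minus its own location, with Y zeroed.
; It rebuilds a separate Route actor's spline with a raised midpoint, and a timeline moves it along the length before both actors are destroyed.
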(event `self.ReceiveBeginPlay`
  (bind (_returnvalue_x _returnvalue_y _returnvalue_z) (`KismetMathLibrary.BreakVector` (`self.K2_GetActorLocation`)))
  (bind _worldlocation (`PlayerController.DeprojectMousePositionToWorld` (`GameplayStatics.GetPlayerController` 0)))
  (set `self.damage` 100.0)
  (bind _output_get (set `self.endLoc` (`KismetMathLibrary.MakeVector` (- (.x _worldlocation) _returnvalue_x) 0.0 (- (.z _worldlocation) _returnvalue_z))))
  (bind _output_get_2 (set `self.startLoc` (`self.K2_GetActorLocation`)))
  (`self.UpdateSpline` _output_get_2 _output_get)
  (`self.moveMissle`))

(event `UpdateSpline`
  (params (startLoc :type "Vector Structure") (endLoc :type "Vector Structure"))
  (`SplineComponent.SetSplinePoints` (`/Game/Blueprint/Tower/Track_BluePrint.Spline_route` (`self.route`)) (`|MakeArray` startLoc (+ (/ (+ startLoc endLoc) 2.0) (0.0 0.0 300.0)) endLoc) "World" true))

(event `moveMissle`
  (bind (_direction _temp) (`Timeline|타임라인_0`)
    (:`Update`
      (set `self.alpha` _temp)
      (`self.K2_SetActorLocation` (`SplineComponent.GetLocationAtDistanceAlongSpline` (`/Game/Blueprint/Tower/Track_BluePrint.Spline_route` (`self.route`)) (`KismetMathLibrary.Lerp` 0.0 (`SplineComponent.GetSplineLength` (`/Game/Blueprint/Tower/Track_BluePrint.Spline_route` (`self.route`))) (`self.alpha`)) "World")))
    (:`Finished`
      (`self.K2_DestroyActor`)
      (`self.K2_DestroyActor` (`self.route`)))))

(fn `UserConstructionScript`)