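; Guided missile tower Blueprint that builds on parent tower logic and fires homing-named missiles at an enemy target, with its own starting HP.
; Each Tick fires when the target is valid and the reload flag is set, or calls TargetNewEnemy when no target is valid and CheckTarget is false.
; Shoot spawns a GuidedMissle_BluePrint given the tower, target and attack sphere radius, then uses a FireRate delay to gate reloading.
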(event `self.ReceiveBeginPlay`
  (set `self.HP` 180.0))

(event `Shoot`
  (`|SpawnActorFromClass` "/Game/Blueprint/Tower/GuidedMissle_BluePrint.GuidedMissle_BluePrint_C" (`self.GetTransform`) "Undefined" "OverrideRootScale" null self (`self.Target`) (`SphereComponent.SphereRadius` (`self.attackRange`)) null)
  (set `self.isReload` false)
  (`KismetSystemLibrary.Delay` (`self.fireRate`))
  (set `self.isReload` true))

(event `self.ReceiveTick`
  (params (DeltaSeconds :type "Float (single-precision)"))
  (`parent.ReceiveTick` DeltaSeconds)
  (`/Engine/EditorBlueprintResources/StandardMacros.IsValid` (`self.Target`)
    (:`Is Valid`
      (if (`self.isReload`)
        (`self.Shoot`)))
    (:`Is Not Valid`
      (if (not (`self.checkTarget`))
        (`self.TargetNewEnemy`)))))

(fn `UserConstructionScript`
  (`parent.UserConstructionScript`))