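; Tower range-selection cursor: a sprite actor that follows the mouse so the player can pick a location within range of a tower.
; Each tick it moves to the deprojected mouse position on a fixed-Y plane and measures XZ distance from its spawn location, stored as the tower location.
; The sprite turns red beyond Range and green otherwise.
; Clicking while green stores SelectLoc and sets IsClicked.
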(event `self.ReceiveBeginPlay`
  (set `self.towerLoc` (`self.K2_GetActorLocation`)))

(event `self.ReceiveTick`
  (params (DeltaSeconds :type "Float (single-precision)"))
  (bind (_towerloc_x _towerloc_y _towerloc_z) (`KismetMathLibrary.BreakVector` (`self.towerLoc`)))
  (bind _worldlocation (`PlayerController.DeprojectMousePositionToWorld` (`GameplayStatics.GetPlayerController` 0)))
  (bind _worldlocation_2 (`PlayerController.DeprojectMousePositionToWorld` (`GameplayStatics.GetPlayerController` 0)))
  (`self.K2_SetActorLocation` (`KismetMathLibrary.MakeVector` (.x _worldlocation) -0.5 (.z _worldlocation)))
  (if (> (`KismetMathLibrary.VSize` (- (`KismetMathLibrary.MakeVector` _towerloc_x 0.0 _towerloc_z) (`KismetMathLibrary.MakeVector` (.x _worldlocation_2) 0.0 (.z _worldlocation_2)))) (`self.range`))
    (`PaperSpriteComponent.SetSprite` (`self.Sprite`) "/Game/Sprite/red_circle_Sprite.red_circle_Sprite")
    (else
      (`PaperSpriteComponent.SetSprite` (`self.Sprite`) "/Game/Sprite/green_circle_Sprite.green_circle_Sprite"))))

(event `self.Sprite.OnClicked`
  (params (TouchedComponent :type "PrimitiveComponent Object Reference") (ButtonPressed :type "Key Structure"))
  (bind _worldlocation (`PlayerController.DeprojectMousePositionToWorld` (`GameplayStatics.GetPlayerController` 0)))
  (if (== (`PaperSpriteComponent.GetSprite` (`self.Sprite`)) "/Game/Sprite/green_circle_Sprite.green_circle_Sprite")
    (set `self.selectLoc` (`KismetMathLibrary.MakeVector` (.x _worldlocation) -0.5 (.z _worldlocation)))
    (set `self.isClicked` true)))

(fn `UserConstructionScript`)