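; The player's ark: a grid map of structures built on a raft, which carries rescued animals.
; Tick rocks it around a lean set by horizontal balance, with random swing scaled by vertical balance.
; On destruction, a recursive flood fill from the origin finds disconnected pieces and drops them with physics.
; Runs of three fences form up to five animal pens, re-placed after collapses; filling all five opens the ending level.
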(event `self.ReceiveBeginPlay`
  (bind _returnvalue (`GameplayStatics.GetActorOfClass` "/Game/Blueprint/Structure/Raft_Blueprint.Raft_Blueprint_C"))
  (bind _output_get (set `self.Raft` _returnvalue))
  (set `self.StructureMap` (`|MakeMap` (-2.0 0.0) _output_get (-1.0 0.0) _output_get (0.0 0.0) _output_get (1.0 0.0) _output_get (2.0 0.0) _output_get :!type "Vector2D Structure" :!valuetype "/Game/Blueprint/Structure/Structure_Blueprint Object Reference"))
  (bind _returnvalue_2 (`GameplayStatics.GetActorOfClass` "/Game/Blueprint/Architect_Blueprint.Architect_Blueprint_C"))
  (set `self.Architect` _returnvalue_2)
  (bind _returnvalue_3 (`GameplayStatics.GetActorOfClass` "/Game/Blueprint/Player_Blueprint.Player_Blueprint_C"))
  (set `self.Player` _returnvalue_3)
  (set `PlayerController.bShowMouseCursor` true (`GameplayStatics.GetPlayerController` 0))
  (set `self.CatFlipbook` "/Game/Sprite/animals/cat/cat_Idle.cat_Idle"))

(event `self.ReceiveTick`
  (params (DeltaSeconds :type "Float (single-precision)"))
  (bind (_returnvalue_roll _returnvalue_pitch) (`KismetMathLibrary.BreakRotator` (`self.K2_GetActorRotation`)))
  (bind (_returnvalue_roll_2 _returnvalue_pitch_2) (`KismetMathLibrary.BreakRotator` (`self.K2_GetActorRotation`)))
  (bind _returnvalue (+ (* (`self.RotationBoundOffset`) (`self.RotationDirection`)) (`KismetMathLibrary.FClamp` (* (`self.HorizontalBalance`) -1.0) -45.0 45.0)))
  (set `self.RotationSpeed` (`KismetMathLibrary.FClamp` (`KismetMathLibrary.Abs` (- _returnvalue_pitch _returnvalue)) 3.0 10.0))
  (if (> (`self.RotationDirection`) 0.0)
    (if (> _returnvalue_pitch _returnvalue)
      (set `self.RotationDirection` (* (`self.RotationDirection`) -1.0) :!label _label)
      (set `self.RotationBoundOffset` (`KismetMathLibrary.RandomFloatInRange` 0.0 (`KismetMathLibrary.FClamp` (`self.VerticalBalance`) 3.0 30.0)))
      (else
        (`self.K2_AddActorWorldRotation` (`KismetMathLibrary.MakeRotator` 0.0 (* (`self.RotationSpeed`) (`self.RotationDirection`) (`GameplayStatics.GetWorldDeltaSeconds`))) :!label _label_2)
        (if (> (`KismetMathLibrary.Abs` _returnvalue_pitch_2) 20.0)
          (`|ExecutionSequence`
            (:`then_0`
              (`/Engine/EditorBlueprintResources/StandardMacros.DoOnce` false
                (:`Completed`
                  (bind _returnvalue_2 (`|CreateWidget` "/Game/Blueprint/UI/Help_ArcList.Help_ArcList_C"))
                  (`UserWidget.AddToViewport` _returnvalue_2 0))))
            (:`then_1`
              (`/Engine/EditorBlueprintResources/StandardMacros.DoOnce` false :!label _label_3
                (:`Completed`
                  (if (> (`KismetMathLibrary.RandomFloat`) 0.5)
                    (`GameplayStatics.PlaySound2D` "/Game/Sound/ship_2.ship_2" 1.0 1.0 0.0 null null)
                    (else
                      (`GameplayStatics.PlaySound2D` "/Game/Sound/ship_1.ship_1" 1.0 1.0 0.0 null null)))
                  (`KismetSystemLibrary.Delay` (`KismetMathLibrary.RandomFloatInRange` 5.0 2.0))
                  (goto _label_3 :!via `Reset`))))))))
    (elif (< _returnvalue_pitch _returnvalue)
      (goto _label)
      (else
        (goto _label_2)))))

(event `StructureDestroyed`
  (params (GridPos :type "Vector2D Structure"))
  (bind _returnvalue (`KismetMathLibrary.RandomFloatInRange` -3000.0 3000.0))
  (bind _structuremap (`self.StructureMap`))
  (bind _structuremap_2 (`self.StructureMap`))
  (bind _gridsize (`/Game/Blueprint/Architect_Blueprint.GridSize` (`self.Architect`)))
  (`BlueprintMapLibrary.Map_Remove` _structuremap_2 GridPos)
  (set `self.AttachedStructureKeys` (`|MakeArray` (0.0 0.0) :!type "Vector2D Structure"))
  (`self.FindAttachedStructure` (0.0 0.0))
  (bind _keys (`BlueprintMapLibrary.Map_Keys` _structuremap_2))
  (for _array_element _keys
    (if (not (`KismetArrayLibrary.Array_Contains` (`self.AttachedStructureKeys`) _array_element))
      (bind _value (`BlueprintMapLibrary.Map_Find` _structuremap _array_element))
      (`self.K2_DetachFromActor` _value "KeepWorld" "KeepWorld" "KeepWorld")
      (`self.SetLifeSpan` _value 3.0)
      (bind _rendercomponent (`PaperSpriteActor.RenderComponent` _value))
      (`PrimitiveComponent.SetSimulatePhysics` _rendercomponent true)
      (`PrimitiveComponent.AddImpulseAtLocation` _rendercomponent (`KismetMathLibrary.MakeVector` _returnvalue 0.0 _returnvalue) (+ (`SceneComponent.K2_GetComponentLocation` _rendercomponent) (`KismetMathLibrary.MakeVector` (`KismetMathLibrary.RandomFloatInRange` (* _gridsize -0.5) (* _gridsize 0.5)))) "None")
      (`self.SetActorEnableCollision` _value false)
      (`BlueprintMapLibrary.Map_Remove` _structuremap _array_element)
      (`self.UpdateBalance`)
      (`self.CheckFence`)
      (`self.RelocateAnimal`))))

(event `StructureConstructed`
  (params (GridPos :type "Vector2D Structure") (Structure :type "/Game/Blueprint/Structure/Structure_Blueprint Object Reference"))
  (`BlueprintMapLibrary.Map_Add` (`self.StructureMap`) GridPos Structure)
  (`self.UpdateBalance`)
  (`self.CheckFence`))

(fn `AddAnimal`
  (params (Animal :type "/Game/Blueprint/Animal_Enum Enum" :default "NewEnumerator0"))
  (returns (Result :type Boolean))
  (bind _returnvalue (select `/Game/Blueprint/Animal_Enum` Animal :`NewEnumerator0` (`self.PaperFlipbook_Cat`) :`NewEnumerator1` (`self.PaperFlipbook_Dog`) :`NewEnumerator2` (`self.PaperFlipbook_Elephant`) :`NewEnumerator3` (`self.PaperFlipbook_Giraffe`) :`NewEnumerator4` (`self.PaperFlipbook_Lion`)))
  (if (not (`KismetArrayLibrary.Array_Contains` (`self.Animals`) Animal))
    (for (_array_element _array_index) (`self.IsFenceEmpty`)
      (if _array_element
        (bind _output (`|GetArrayItem` (`self.FencePosition`) _array_index))
        (if (!= _output (0.0 0.0))
          (`KismetArrayLibrary.Array_Set` (`self.Animals`) _array_index Animal)
          (`KismetArrayLibrary.Array_Set` (`self.IsFenceEmpty`) _array_index)
          (bind (_returnvalue_x _returnvalue_y) (`KismetMathLibrary.BreakVector2D` (* (+ _output (1.0 0.0)) (`/Game/Blueprint/Architect_Blueprint.GridSize` (`self.Architect`)))))
          (`SceneComponent.K2_SetRelativeLocation` _returnvalue (`KismetMathLibrary.MakeVector` _returnvalue_x -1.0 _returnvalue_y) false false)
          (`PaperFlipbookComponent.SetSpriteColor` _returnvalue (make `LinearColor` 1.0 1.0 1.0 1.0))
          (`GameplayStatics.PlaySound2D` (select `/Game/Blueprint/Animal_Enum` Animal :`NewEnumerator0` "/Game/Sound/cat.cat" :`NewEnumerator1` "/Game/Sound/dog.dog" :`NewEnumerator2` "/Game/Sound/elephant.elephant" :`NewEnumerator3` "/Game/Sound/giraffe.giraffe" :`NewEnumerator4` "/Game/Sound/lion.lion" :!type "SoundBase Object Reference") 1.0 1.0 0.0 null null)
          (for _array_element_2 (`self.IsFenceEmpty`)
            (if _array_element_2
              (return true)))
          (`GameplayStatics.OpenLevel` "Ending_Lobby")))))
  (return false))

(fn `CheckFence`
  (locals (FoundFail :type Boolean) (Exist :type Boolean))
  (bind _structuremap (`self.StructureMap`))
  (set `self.FencePosition` (`|MakeArray` (0.0 0.0) (0.0 0.0) (0.0 0.0) (0.0 0.0) (0.0 0.0) :!type "Vector2D Structure"))
  (bind _keys (`BlueprintMapLibrary.Map_Keys` _structuremap))
  (for _array_element _keys
    (if (== (`GameplayStatics.GetObjectClass` (`BlueprintMapLibrary.Map_Find` _structuremap _array_element)) "/Game/Blueprint/Structure/Fence_Blueprint.Fence_Blueprint_C")
      (set `local.Exist` false)
      (for _array_element_2 (`self.FencePosition`) :!label _label
        (for _array_element_3 (`|MakeArray` (1.0 0.0) (2.0 0.0) (0.0 0.0) :!type "Vector2D Structure")
          (if (== (+ _array_element_3 _array_element_2) _array_element)
            (set `local.Exist` true)
            (goto _label :!via `Break`))))
      (if (not (`local.Exist`))
        (set `local.FoundFail` false)
        (for _array_element_4 (`|MakeArray` (1.0 0.0) (2.0 0.0) :!type "Vector2D Structure")
          (bind (_value _returnvalue) (`BlueprintMapLibrary.Map_Find` (`self.StructureMap`) (+ _array_element_4 _array_element)))
          (if _returnvalue
            (if (not (== (`GameplayStatics.GetObjectClass` _value) "/Game/Blueprint/Structure/Fence_Blueprint.Fence_Blueprint_C"))
              (set `local.FoundFail` true :!label _label_2)
              (break))
            (else
              (goto _label_2))))
        (if (not (`local.FoundFail`))
          (for (_array_element_5 _array_index) (`self.FencePosition`)
            (if (== _array_element_5 (0.0 0.0))
              (`KismetArrayLibrary.Array_Set` (`self.FencePosition`) _array_index _array_element)
              (break))))))))

(fn `FindAttachedStructure`
  (params (Element :type "Vector2D Structure"))
  (for _array_element (`|MakeArray` (-1.0 0.0) (1.0 0.0) (0.0 -1.0) (0.0 1.0) :!type "Vector2D Structure")
    (bind _returnvalue (+ Element _array_element))
    (if (not (`KismetArrayLibrary.Array_Contains` (`self.AttachedStructureKeys`) _returnvalue))
      (bind _keys (`BlueprintMapLibrary.Map_Keys` (`self.StructureMap`)))
      (if (`KismetArrayLibrary.Array_Contains` _keys _returnvalue)
        (`KismetArrayLibrary.Array_Add` (`self.AttachedStructureKeys`) _returnvalue)
        (`self.FindAttachedStructure` _returnvalue))))
  (return))

(fn `GetRelativeMousePos`
  (returns (Position :type "Vector2D Structure"))
  (bind _returnvalue (`KismetMathLibrary.MakeRelativeTransform` (`KismetMathLibrary.MakeTransform` (`PlayerController.DeprojectMousePositionToWorld` (`GameplayStatics.GetPlayerController` 0))) (`self.GetTransform`)))
  (return (`KismetMathLibrary.MakeVector2D` (.x (.location _returnvalue)) (.z (.location _returnvalue)))))

(fn `RelocateAnimal`
  (locals (NewAnimals :type "Array of /Game/Blueprint/Animal_Enum Enum"))
  (for _array_element (`|MakeArray` (`self.PaperFlipbook_Cat`) (`self.PaperFlipbook_Dog`) (`self.PaperFlipbook_Elephant`) (`self.PaperFlipbook_Giraffe`) (`self.PaperFlipbook_Lion`))
    (`PaperFlipbookComponent.SetSpriteColor` _array_element (make `LinearColor` 1.0 1.0 1.0)))
  (set `self.IsFenceEmpty` (`|MakeArray` true true true true true))
  (for (_array_element_2 _array_index) (`self.Animals`)
    (if (`|EnumInequality` _array_element_2 "NewEnumerator5")
      (bind _output (`|GetArrayItem` (`self.FencePosition`) _array_index))
      (if (and (!= _output (0.0 0.0)) (`|GetArrayItem` (`self.IsFenceEmpty`) _array_index))
        (`KismetArrayLibrary.Array_Set` (`local.NewAnimals`) _array_index _array_element_2)
        (`KismetArrayLibrary.Array_Set` (`self.IsFenceEmpty`) _array_index)
        (bind _returnvalue (select `/Game/Blueprint/Animal_Enum` _array_element_2 :`NewEnumerator0` (`self.PaperFlipbook_Cat`) :`NewEnumerator1` (`self.PaperFlipbook_Dog`) :`NewEnumerator2` (`self.PaperFlipbook_Elephant`) :`NewEnumerator3` (`self.PaperFlipbook_Giraffe`) :`NewEnumerator4` (`self.PaperFlipbook_Lion`)))
        (bind (_returnvalue_x _returnvalue_y) (`KismetMathLibrary.BreakVector2D` (* (+ _output (1.0 0.0)) (`/Game/Blueprint/Architect_Blueprint.GridSize` (`self.Architect`)))))
        (`SceneComponent.K2_SetRelativeLocation` _returnvalue (`KismetMathLibrary.MakeVector` _returnvalue_x -1.0 _returnvalue_y) false false)
        (`PaperFlipbookComponent.SetSpriteColor` _returnvalue (make `LinearColor` 1.0 1.0 1.0 1.0)))))
  (set `self.Animals` (`local.NewAnimals`)))

(fn `UpdateBalance`
  (set `self.HorizontalBalance` 0.0)
  (set `self.VerticalBalance` 0.0)
  (bind _keys (`BlueprintMapLibrary.Map_Keys` (`self.StructureMap`)))
  (for _array_element _keys
    (bind (_x _y) (`KismetMathLibrary.BreakVector2D` _array_element))
    (set `self.HorizontalBalance` (+ _x (`self.HorizontalBalance`)))
    (set `self.VerticalBalance` (+ (`self.VerticalBalance`) (- (`KismetMathLibrary.Abs` _y) (`KismetMathLibrary.Abs` _x))))))

(fn `UserConstructionScript`)