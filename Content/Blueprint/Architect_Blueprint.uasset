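; Architect is the cursor actor, attached to the Arc, that places and demolishes structures on its grid.
; Each tick it snaps to the mouse's grid cell, with a preview sprite set by SetStructureType and tinted red on overlap.
; A click builds in a free cell adjacent to an existing structure if Player.MixItem accepts the cost, registering it with the Arc.
; In destroy mode, a click deals lethal damage to any structure except the Raft.
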(event `self.ReceiveActorEndOverlap`
  (params (OtherActor :type "Actor Object Reference"))
  (if (`|EnumEquality` (`self.ArchitectState`) "NewEnumerator0")
    (set `self.IsOverlap` false)
    (`PaperSpriteComponent.SetSpriteColor` (`self.RenderComponent`) (make `LinearColor` 255.0 255.0 255.0 0.7))))

(event `self.ReceiveActorBeginOverlap`
  (params (OtherActor :type "Actor Object Reference"))
  (if (`|EnumEquality` (`self.ArchitectState`) "NewEnumerator0")
    (set `self.IsOverlap` true)
    (`PaperSpriteComponent.SetSpriteColor` (`self.RenderComponent`) (make `LinearColor` 255.0 0.0 0.0 0.7))))

(event `Key|LeftMouseButton` :consume false
  (params (Key :type "Key Structure"))
  (bind (_gridpos_x _gridpos_y) (`KismetMathLibrary.BreakVector2D` (`self.GridPos`)))
  (bind _architectstate (`self.ArchitectState`))
  (bind _gridpos (`self.GridPos`))
  (bind (_returnvalue_location _returnvalue_rotation _returnvalue_scale) (`KismetMathLibrary.BreakTransform` (`SceneComponent.GetRelativeTransform` (`self.RenderComponent`))))
  (bind (_value _returnvalue) (`BlueprintMapLibrary.Map_Find` (`/Game/Blueprint/Arc_Blueprint.StructureMap` (`self.Arc`)) (`self.GridPos`)))
  (:`Pressed`
    (if (`|EnumEquality` _architectstate "NewEnumerator1")
      (if _returnvalue
        (if (!= _value (`/Game/Blueprint/Arc_Blueprint.Raft` (`self.Arc`)))
          (`/Game/Blueprint/Structure/Structure_Blueprint.Damaged` _value 99999.0)))
      (elif (and (`|EnumEquality` _architectstate "NewEnumerator0") (> _gridpos_y -2.0))
        (if (not (`self.IsOverlap`))
          (bind _keys (`BlueprintMapLibrary.Map_Keys` (`/Game/Blueprint/Arc_Blueprint.StructureMap` (`self.Arc`))))
          (if (and (not (`KismetArrayLibrary.Array_Contains` _keys _gridpos)) (or (`KismetArrayLibrary.Array_Contains` _keys (+ _gridpos (-1.0 0.0))) (`KismetArrayLibrary.Array_Contains` _keys (+ _gridpos (1.0 0.0))) (`KismetArrayLibrary.Array_Contains` _keys (+ _gridpos (0.0 -1.0))) (`KismetArrayLibrary.Array_Contains` _keys (+ _gridpos (0.0 1.0)))))
            (bind _cost (`/Game/Blueprint/Structure/StructureInfo_Blueprint.GetStructureCost` (`self.StructureInfo`) (`self.StructureType`)))
            (bind _success (`/Game/Blueprint/Player_Blueprint.Mix Item` (`/Game/Blueprint/Arc_Blueprint.Player` (`self.Arc`)) _cost))
            (if _success
              (bind _returnvalue_2 (`|SpawnActorFromClass` (select `/Game/Blueprint/Structure/Structure_Enum` (`self.StructureType`) :`NewEnumerator0` "/Game/Blueprint/Structure/WoodBlock_Blueprint.WoodBlock_Blueprint_C" :`NewEnumerator2` "/Game/Blueprint/Structure/WoodLadder_Blueprint.WoodLadder_Blueprint_C" :`NewEnumerator3` "/Game/Blueprint/Structure/Chest_Blueprint.Chest_Blueprint_C" :`NewEnumerator1` "/Game/Blueprint/Tower/NormalTower_BluePrint.NormalTower_BluePrint_C" :`NewEnumerator9` "/Game/Blueprint/Tower/GuidedTower_BluePRint.GuidedTower_BluePRint_C" :`NewEnumerator4` "/Game/Blueprint/Structure/StoneBlock_Blueprint.StoneBlock_Blueprint_C" :`NewEnumerator5` "/Game/Blueprint/Structure/CopperBlock_Blueprint.CopperBlock_Blueprint_C" :`NewEnumerator6` "/Game/Blueprint/Structure/SilverBlock_Blueprint.SilverBlock_Blueprint_C" :`NewEnumerator7` "/Game/Blueprint/Structure/GoldBlock_Blueprint.GoldBlock_Blueprint_C" :`NewEnumerator8` "/Game/Blueprint/Structure/Fence_Blueprint.Fence_Blueprint_C" :`NewEnumerator10` "/Game/Blueprint/Structure/Crane_Blueprint.Crane_Blueprint_C" :!type "/Game/Blueprint/Structure/Structure_Blueprint Class Reference") (`KismetMathLibrary.MakeTransform` (+ _returnvalue_location (0.0 -1.0 0.0)) _returnvalue_rotation _returnvalue_scale) "Undefined" "OverrideRootScale" null null))
              (bind _maxhp (`/Game/Blueprint/Structure/StructureInfo_Blueprint.GetStructureMaxHP` (`self.StructureInfo`) (`self.StructureType`)))
              (`/Game/Blueprint/Structure/Structure_Blueprint.SetMaxHP` _returnvalue_2 _maxhp)
              (set `/Game/Blueprint/Structure/Structure_Blueprint.GridPos` (`self.GridPos`) _returnvalue_2)
              (`self.K2_AttachToActor` _returnvalue_2 (`self.Arc`) "None" "KeepRelative" "KeepRelative" "KeepRelative" true)
              (`/Game/Blueprint/Arc_Blueprint.StructureConstructed` (`self.Arc`) (`self.GridPos`) _returnvalue_2)
              (`GameplayStatics.PlaySound2D` "/Game/Sound/block_const.block_const" 1.0 1.0 0.0 null null)
              (else
                (bind _returnvalue_3 (`|CreateWidget` "/Game/Blueprint/UI/MessageWidget_Blueprint.MessageWidget_Blueprint_C"))
                (`UserWidget.AddToViewport` _returnvalue_3 0)
                (`/Game/Blueprint/UI/MessageWidget_Blueprint.SetText` _returnvalue_3 "자원이 부족합니다")))))))))

(event `self.ReceiveBeginPlay`
  (bind _asarc_blueprint (cast `/Game/Blueprint/Arc_Blueprint` (`self.GetAttachParentActor`)))
  (set `self.Arc` _asarc_blueprint)
  (bind _returnvalue (`GameplayStatics.GetActorOfClass` "/Game/Blueprint/Structure/StructureInfo_Blueprint.StructureInfo_Blueprint_C"))
  (set `self.StructureInfo` _returnvalue))

(event `self.ReceiveTick`
  (params (DeltaSeconds :type "Float (single-precision)"))
  (bind (_dividedmousepos_x _dividedmousepos_y) (`KismetMathLibrary.BreakVector2D` (`self.DividedMousePos`)))
  (bind _dividedmousepos_x_2 (`KismetMathLibrary.BreakVector2D` (`self.DividedMousePos`)))
  (bind (_relativemousepos_x _relativemousepos_y) (`KismetMathLibrary.BreakVector2D` (`self.RelativeMousePos`)))
  (bind (_dividedmousepos_x_3 _dividedmousepos_y_2) (`KismetMathLibrary.BreakVector2D` (`self.DividedMousePos`)))
  (bind _relativemousepos_x_2 (`KismetMathLibrary.BreakVector2D` (`self.RelativeMousePos`)))
  (bind (_relativemousepos_x_3 _relativemousepos_y_2) (`KismetMathLibrary.BreakVector2D` (`self.RelativeMousePos`)))
  (bind (_dividedmousepos_x_4 _dividedmousepos_y_3) (`KismetMathLibrary.BreakVector2D` (`self.DividedMousePos`)))
  (bind _returnvalue (/ (`self.GridSize`) 2.0))
  (bind _position (`/Game/Blueprint/Arc_Blueprint.GetRelativeMousePos` (`self.Arc`)))
  (set `self.RelativeMousePos` _position)
  (`|ExecutionSequence`
    (:`then_0`
      (if (> _relativemousepos_x_3 _returnvalue)
        (set `self.DividedMousePos` (`KismetMathLibrary.MakeVector2D` (+ _relativemousepos_x_2 (`self.GridSize`)) _dividedmousepos_y_2))
        (else
          (set `self.DividedMousePos` (`KismetMathLibrary.MakeVector2D` _relativemousepos_x_2 _dividedmousepos_y_2)))))
    (:`then_1`
      (if (> _relativemousepos_y_2 _returnvalue)
        (set `self.DividedMousePos` (`KismetMathLibrary.MakeVector2D` _dividedmousepos_x_2 (+ _relativemousepos_y (`self.GridSize`))))
        (else
          (set `self.DividedMousePos` (`KismetMathLibrary.MakeVector2D` _dividedmousepos_x_2 _relativemousepos_y))))
      (`|ExecutionSequence`
        (:`then_0`
          (bind _dividedvalue (`self.DivideByGridSize` _dividedmousepos_x_4))
          (set `self.DividedMousePos` (`KismetMathLibrary.MakeVector2D` _dividedvalue _dividedmousepos_y)))
        (:`then_1`
          (bind _dividedvalue_2 (`self.DivideByGridSize` _dividedmousepos_y_3))
          (bind _output_get (set `self.DividedMousePos` (`KismetMathLibrary.MakeVector2D` _dividedmousepos_x _dividedvalue_2)))
          (`self.K2_SetActorRelativeLocation` (`KismetMathLibrary.MakeVector` (`KismetMathLibrary.BreakVector2D` _output_get) 0.0 (`.Y` (`KismetMathLibrary.BreakVector2D` _output_get))))
          (set `self.GridPos` (`KismetMathLibrary.ToRounded2D` (/ (`self.DividedMousePos`) (`self.GridSize`)))))))))

(fn `DivideByGridSize`
  (params (Value :type "Float (double-precision)"))
  (returns (DividedValue :type "Float (double-precision)"))
  (bind _returnvalue (`KismetMathLibrary.FTrunc` (`self.GridSize`)))
  (return (`KismetMathLibrary.Conv_IntToDouble` (* (/ (- (`KismetMathLibrary.FTrunc` Value) (/ _returnvalue 2)) _returnvalue) _returnvalue))))

(fn `SetStructureType`
  (params (Type :type "/Game/Blueprint/Structure/Structure_Enum Enum" :default "NewEnumerator0") (Destroy :type Boolean))
  (bind _rendercomponent (`self.RenderComponent`))
  (if Destroy
    (set `self.ArchitectState` "NewEnumerator1")
    (`PaperSpriteComponent.SetSprite` _rendercomponent "/Game/Texture/Icon/x_button_Sprite.x_button_Sprite")
    (`PaperSpriteComponent.SetSpriteColor` _rendercomponent (struct :`R` 1.0 :`G` 1.0 :`B` 1.0 :`A` 0.5))
    (`/Engine/EditorBlueprintResources/StandardMacros.DoOnce` false
      (:`Completed`
        (bind _returnvalue (`|CreateWidget` "/Game/Blueprint/UI/Help_Destroy.Help_Destroy_C"))
        (`UserWidget.AddToViewport` _returnvalue 0)))
    (else
      (bind _output_get (set `self.StructureType` Type))
      (`PaperSpriteComponent.SetSprite` (`self.RenderComponent`) (select `/Game/Blueprint/Structure/Structure_Enum` _output_get :`NewEnumerator0` "/Game/Sprite/blocks/wood_block_Sprite.wood_block_Sprite" :`NewEnumerator2` "/Game/Sprite/WoodLadder_Sprite.WoodLadder_Sprite" :`NewEnumerator3` "/Game/Sprite/blocks/chest_Sprite.chest_Sprite" :`NewEnumerator1` "/Game/Sprite/tower/parabola_cannon/cannon+wheel_Sprite.cannon+wheel_Sprite" :`NewEnumerator9` "/Game/Sprite/tower/guided_cannon/g_cannon_Sprite.g_cannon_Sprite" :`NewEnumerator4` "/Game/Sprite/blocks/stone_block_Sprite.stone_block_Sprite" :`NewEnumerator5` "/Game/Sprite/blocks/copper_block_Sprite.copper_block_Sprite" :`NewEnumerator6` "/Game/Sprite/blocks/silver_block_Sprite.silver_block_Sprite" :`NewEnumerator7` "/Game/Sprite/blocks/gold_block_Sprite.gold_block_Sprite" :`NewEnumerator8` "/Game/Sprite/blocks/fence_Sprite.fence_Sprite" :`NewEnumerator10` "/Game/Sprite/blocks/crane_Sprite.crane_Sprite" :!type "PaperSprite Object Reference"))
      (set `self.ArchitectState` "NewEnumerator0")
      (set `self.IsOverlap` (`self.IsOverlappingActor` null)))))

(fn `UserConstructionScript`)