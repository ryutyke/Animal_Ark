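; IntroManager drives the story intro, a narrated prologue about a flooded world and a raft, then opens the main_ArcTest level.
; On BeginPlay it creates the intro widget, registers itself with it, fills parallel text, voice and delay arrays, and starts background music.
; NextStep advances through them, showing the next-text prompt after each delay.
; A DoOnce blocks repeat advances until each line's delay ends.
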(event `self.ReceiveBeginPlay`
  (bind _returnvalue (`|CreateWidget` "/Game/Blueprint/IntroWidget_Blueprint.IntroWidget_Blueprint_C"))
  (bind _output_get (set `self.IntroWidget` _returnvalue))
  (`UserWidget.AddToViewport` _output_get 0)
  (set `self.Dialogues` (`|MakeArray` "2038년, 태평양에 거대한 운성이 떨어졌고 온 세상은 물에 잠겼습니다." "거대한 파도가 덮쳐오는 순간, 당신은 신에게 구해달라고 기도를 빌었습니다." "잠시 후 눈을 떠보니, 당신의 눈 앞에 뗏목이 생겼습니다." "이 뗏목은 절대 가라않지 않았지만, 당신의 영혼이 묶여있는 느낌을 받았습니다." "조심하세요. 당신은 죽어도 뗏목에서 부활하지만, 뗏목이 부서지면 당신도 죽게 됩니다." "종말의 상황에서 방주를 만들고 최대한 많은 생명을 구해보십시오."))
  (set `/Game/Blueprint/IntroWidget_Blueprint.IntroManager` self _output_get)
  (set `self.Sound` (`|MakeArray` "/Game/Sound/Intro/Arc_Intro_part1.Arc_Intro_part1" "/Game/Sound/Intro/Arc_Intro_part2.Arc_Intro_part2" "/Game/Sound/Intro/Arc_Intro_part3.Arc_Intro_part3" "/Game/Sound/Intro/Arc_Intro_part4.Arc_Intro_part4" "/Game/Sound/Intro/Arc_Intro_part5.Arc_Intro_part5" "/Game/Sound/Intro/Arc_Intro_part6.Arc_Intro_part6" :!type "SoundWave Object Reference"))
  (set `self.SoundDelay` (`|MakeArray` 7.5 5.1 6.1 5.9 8.0 6.8 :!type "Float (single-precision)"))
  (set `PlayerController.bShowMouseCursor` true (`GameplayStatics.GetPlayerController` 0))
  (`GameplayStatics.PlaySound2D` "/Game/Sound/FantasyOrchestral/cues/EpicFantasy.EpicFantasy" 3.0 1.0 0.0 null null))

(event `NextStep`
  (`/Engine/EditorBlueprintResources/StandardMacros.DoOnce` false :!label _label
    (:`Completed`
      (`/Game/Blueprint/IntroWidget_Blueprint.ShowNextText` (`self.IntroWidget`) false)
      (bind _output_get (set `self.Step` (+ (`self.Step`) 1)))
      (if (> _output_get 5)
        (`self.PlayGame`)
        (else
          (`/Game/Blueprint/IntroWidget_Blueprint.SetScreenText` (`self.IntroWidget`) (`|GetArrayItem` (`self.Dialogues`) (`self.Step`)))
          (`GameplayStatics.PlaySound2D` (`|GetArrayItem` (`self.Sound`) (`self.Step`)) 5.0 1.0 0.0 null null)
          (`KismetSystemLibrary.Delay` (`|GetArrayItem` (`self.SoundDelay`) (`self.Step`)))
          (`/Game/Blueprint/IntroWidget_Blueprint.ShowNextText` (`self.IntroWidget`) true)
          (goto _label :!via `Reset`))))))

(event `PlayGame`
  (`GameplayStatics.OpenLevel` "main_ArcTest"))

(fn `UserConstructionScript`)