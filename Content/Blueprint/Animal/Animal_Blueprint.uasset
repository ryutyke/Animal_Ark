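; Animal actor Blueprint that drifts along the world X axis at a random speed chosen on BeginPlay.
; Each Tick adds that speed to the actor's location without sweep or delta-time scaling, so movement ignores collision and depends on frame rate.
; Interact handlers are empty stubs, and UseItem only returns true.
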(event `self.ReceiveBeginPlay`
  (set `self.speed` (`KismetMathLibrary.RandomFloat`)))

(event `self.ReceiveTick`
  (params (DeltaSeconds :type "Float (single-precision)"))
  (`self.K2_SetActorLocation` (+ (`self.K2_GetActorLocation`) (`KismetMathLibrary.MakeVector` (`self.speed`)))))

(event `Interact_1_3`
  (params (Interacter :type "Actor Object Reference")))

(fn `Interact`
  (params (Interacter :type "Actor Object Reference"))
  (return))

(fn `UseItem`
  (returns (Success :type Boolean))
  (return true))

(fn `UserConstructionScript`)